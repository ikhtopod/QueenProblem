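; BP_StandButton is an interactable stand button in the queen problem game that tells the main chessboard to update its queen positions.
; On BeginPlay it finds and caches a Chessboard_BP actor tagged MainChessboard, printing an error if none is found or the reference is invalid.
; Interacting with the button calls UpdatePositionOfQueens on that cached chessboard.
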(event EventInteract
  (Default|UpdatePositionOfQueens (Variables|Default|GetMainChessboard)))

(event EventBeginPlay
  (CallFunction|FindMainChessboard))

(fn ConstructionScript)

(fn FindMainChessboard
  (bind _outactors (Actor|GetAllActorsOfClasswithTag "/Game/QueenProblem/BP/Chess/Chessboard_BP.Chessboard_BP_C" "MainChessboard"))
  (if (== (Utilities|Array|Length _outactors) 0)
    (Development|PrintString "Error: MainChessboard not exists!" true true "(R=0.463542,G=0.002574,B=0.000000,A=1.000000)" 5.0)
    (else
      (bind _result (Math|Integer|DecrementInt (Utilities|Array|Length _outactors))
        (:%20%20
          (bind _index (Utilities|FlowControl|ForLoopwithBreak 0 _result :!label _label)
            (:LoopBody
              (bind _aschessboard_bp (Utilities|Casting|CastToChessboard_BP (Utilities|Array|Get(acopy) _outactors _index)))
              (Variables|Default|SetMainChessboard _aschessboard_bp)
              (goto _label Break))
            (:Completed
              (Utilities|IsValid (Variables|Default|GetMainChessboard)
                (:Is%20Valid
                  _)
                (:Is%20Not%20Valid
                  (Development|PrintString "Error: finded not correct class for MainChessboard actor!" true true "(R=0.463542,G=0.002574,B=0.000000,A=1.000000)" 5.0)))))))))
  (return))