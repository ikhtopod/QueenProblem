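; Chessboard actor that sets up a random eight-queens layout when play begins.
; SpawnQueenChilds spawns eight Queen_BP actors, attaches them to the board and stores them in QueenActors.
; QueenRandomLocation then gives each queen its own X line and a random Y cell on a 150-unit grid, set as an actor location rather than a relative one.
; No conflict checking or solving happens here.
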(event EventBeginPlay
  (CallFunction|SpawnQueenChilds)
  (CallFunction|QueenRandomLocation))

(fn ConstructionScript)

(fn SpawnQueenChilds
  (for _index (range 0 7)
    (bind _returnvalue (Game|SpawnActorfromClass "/Game/QueenProblem/BP/Chess/Queen_BP.Queen_BP_C" (Math|Transform|MakeTransform "0, 0, 0") "Undefined" self 0))
    (Utilities|Array|Add (Variables|Default|GetQueenActors) _returnvalue)
    (Transformation|AttachActorToActor _returnvalue self "None" "KeepRelative" "KeepRelative" "KeepRelative" true))
  (return))

(fn QueenRandomLocation
  (bind _result (Math|Integer|DecrementInt (Utilities|Array|Length (Variables|Default|GetQueenActors)))
    (:%20%20
      (for _index (range 0 _result)
        (Transformation|SetActorLocation (Utilities|Array|Get(acopy) (Variables|Default|GetQueenActors) _index) (Math|Vector|MakeVector (* _index 1.5e+02) (* (Math|Random|RandomIntegerinRange 0 _result) 1.5e+02) 0.0) false false))
      (return))))